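; An actor that exercises a UDP component by sending and receiving text over the network.
; It emits a greeting on BeginPlay, then sends the frame's DeltaSeconds as a string converted to bytes on every Tick.
; Incoming bytes from the component's receive event are converted to a string and printed.
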(event OnReceivedBytes(UDP)
  (params (Bytes :type Array%20of%20Bytes) (IPAddress :type String) (Port :type Integer%20%28by%20ref%29))
  (Development|PrintString (Class|CUBlueprintLibrary|ToString(Bytes) Bytes)))

(event EventBeginPlay
  (Class|UDPComponent|EmitBytes (Variables|Default|GetUDP) (Class|CUBlueprintLibrary|ToBytes(String) "hi there!")))

(event Collision|EventActorBeginOverlap
  (params (OtherActor :type Actor%20Object%20Reference)))

(event EventTick
  (params (DeltaSeconds :type Float%20%28single-precision%29))
  (Class|UDPComponent|EmitBytes (Variables|Default|GetUDP) (Class|CUBlueprintLibrary|ToBytes(String) (Utilities|String|ToString(Float) DeltaSeconds))))

(fn ConstructionScript)