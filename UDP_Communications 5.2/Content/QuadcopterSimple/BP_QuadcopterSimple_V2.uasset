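; Quadcopter pawn flown by keyboard axes or by JSON commands received over UDP.
; Axis inputs set one active flag, and a timeline applies that movement, yaw or camera pitch; hover clears the flags.
; Goto, rotate-by-degrees and turn-towards commands use eased MoveComponentTo with speed-derived durations.
; On request it sends back position with collision count, or camera line-trace distance, and it prints received grades.
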(event OnReceivedBytes(UDPComponent)
  (params (Bytes :type Array%20of%20Bytes) (IPAddress :type String) (Port :type Integer%20%28by%20ref%29))
  (bind _branchisactive (Variables|Utility|GetBranchIsActive))
  (bind _branchisactive_2 (Variables|Utility|GetBranchIsActive))
  (bind _branchisactive_3 (Variables|Utility|GetBranchIsActive))
  (bind _branchisactive_4 (Variables|Utility|GetBranchIsActive))
  (bind _branchisactive_5 (Variables|Utility|GetBranchIsActive))
  (bind _quadcopterbox (Variables|Default|GetQuadcopterBox))
  (bind _quadcopterbox_2 (Variables|Default|GetQuadcopterBox))
  (bind _quadcopterbox_3 (Variables|Default|GetQuadcopterBox))
  (bind _branchisactive_6 (Variables|Utility|GetBranchIsActive))
  (bind _camera (Variables|Default|GetCamera))
  (bind _returnvalue (Transformation|GetRelativeTransform _quadcopterbox_2))
  (bind _returnvalue_2 (Transformation|GetWorldRotation _camera))
  (bind _returnvalue_3 (Transformation|GetRelativeTransform _quadcopterbox))
  (bind _returnvalue_4 (Transformation|GetWorldLocation _quadcopterbox_3))
  (bind (_outjsonobject _returnvalue_5) (Class|JsonBlueprintFunctionLibrary|FromString (Class|CUBlueprintLibrary|ToString(Bytes) Bytes)))
  (if _returnvalue_5
    (Variables|Utility|SetInputJson _outjsonobject)
    (Utilities|FlowControl|Sequence
      (:then_0
        ;[0.8565 1 0.7031] Momentary Controls of Quadcopter
        (bind (_outvalue _returnvalue_6) (|GetJsonField (Variables|Utility|GetInputJson) "controls")) ; Handling primitive input
        (if _returnvalue_6
          (Variables|Utility|SetControls _outvalue)
          (Utilities|FlowControl|Sequence
            (:then_0
              ;;[1 1 1] Handling Throttle
              (bind (_outvalue_2 _returnvalue_7) (|GetJsonField (Variables|Utility|GetControls) "upAmount")) ; Input froom JSON received
              (if _returnvalue_7
                (Variables|Utility|SetThrottleAxisValue _outvalue_2)
                ;;[1 1 1] Set all elements of array to false
                (for (_ _array_index) _branchisactive_4
                  (Utilities|Array|SetArrayElem _branchisactive_4 _array_index false))
                (Utilities|Array|SetArrayElem _branchisactive_4 0 true) ; Set the relevant array element to true
                (Timeline|ConstantTime PlayFromStart
                  (:Update
                    (if (Utilities|Array|Get(acopy) (Variables|Utility|GetBranchIsActive))
                      ;;[1 1 1] Movement Control - Throttle
                      (Class|PawnMovementComponent|AddInputVector (Variables|Default|GetFloatingPawnMovement) (* (Variables|Utility|GetThrottleAxisValue) (Math|Vector|VectorUp)) false)
                      (elif (Utilities|Array|Get(acopy) (Variables|Utility|GetBranchIsActive) 1)
                        ;;[1 1 1] Movement Control - Pitch
                        (Class|PawnMovementComponent|AddInputVector (Variables|Default|GetFloatingPawnMovement) (* (Variables|Utility|GetPitchAxisValue) (Transformation|GetActorForwardVector)) false)
                        (elif (Utilities|Array|Get(acopy) (Variables|Utility|GetBranchIsActive) 2)
                          ;;[1 1 1] Movement Control - Roll
                          (Class|PawnMovementComponent|AddInputVector (Variables|Default|GetFloatingPawnMovement) (* (Variables|Utility|GetRollAxisValue) (Transformation|GetActorRightVector)) false)
                          (elif (Utilities|Array|Get(acopy) (Variables|Utility|GetBranchIsActive) 3)
                            ;;[1 1 1] Movement Control - Yaw
                            (Transformation|SetWorldRotation (Variables|Default|GetQuadcopterBox) (Math|Rotator|MakeRotator 0.0 0.0 (+ (* (Variables|Utility|GetYawAxisValue) 3.0) (.yaw (Transformation|GetWorldRotation (Variables|Default|GetQuadcopterBox))))) false false)
                            (elif (Utilities|Array|Get(acopy) (Variables|Utility|GetBranchIsActive) 4)
                              ;;[1 1 1] Movement Control - Camera Pitch
                              (if (< (Math|Float|Absolute(Float) (+ (* (Variables|Utility|GetCameraPitchAxisValue) 2.0) (.pitch _returnvalue_2))) 9e+01)
                                (Transformation|SetWorldRotation (Variables|Default|GetCamera) (Math|Rotator|MakeRotator (.roll _returnvalue_2) (+ (* (Variables|Utility|GetCameraPitchAxisValue) 2.0) (.pitch _returnvalue_2)) (.yaw _returnvalue_2)) false false)))))))))))
            (:then_1
              ;;[1 1 1] Handling Pitch
              (bind (_outvalue_3 _returnvalue_8) (|GetJsonField (Variables|Utility|GetControls) "pitchForwardAmount")) ; Input froom JSON received
              (if _returnvalue_8
                (Variables|Utility|SetPitchAxisValue _outvalue_3)
                ;;[1 1 1] Set all elements of array to false
                (for (_ _array_index_2) _branchisactive
                  (Utilities|Array|SetArrayElem _branchisactive _array_index_2 false))
                (Utilities|Array|SetArrayElem _branchisactive 1 true) ; Set the relevant array element to true
                (Timeline|ConstantTime PlayFromStart)))
            (:then_2
              ;;[1 1 1] Handle Roll
              (bind (_outvalue_4 _returnvalue_9) (|GetJsonField (Variables|Utility|GetControls) "rollRightAmount")) ; Input froom JSON received
              (if _returnvalue_9
                (Variables|Utility|SetRollAxisValue _outvalue_4)
                ;;[1 1 1] Set all elements of array to false
                (for (_ _array_index_3) _branchisactive_2
                  (Utilities|Array|SetArrayElem _branchisactive_2 _array_index_3 false))
                (Utilities|Array|SetArrayElem _branchisactive_2 2 true) ; Set the relevant array element to true
                (Timeline|ConstantTime PlayFromStart)))
            (:then_3
              ;;[1 1 1] Handle Yaw
              (bind (_outvalue_5 _returnvalue_10) (|GetJsonField (Variables|Utility|GetControls) "yawRightAmount")) ; Input froom JSON received
              (if _returnvalue_10
                (Variables|Utility|SetYawAxisValue _outvalue_5)
                ;;[1 1 1] Set all elements of array to false
                (for (_ _array_index_4) _branchisactive_3
                  (Utilities|Array|SetArrayElem _branchisactive_3 _array_index_4 false))
                (Utilities|Array|SetArrayElem _branchisactive_3 3 true) ; Set the relevant array element to true
                (Timeline|ConstantTime PlayFromStart)))
            (:then_4
              ;;[1 1 1] Handle Camera Pitch
              (bind (_outvalue_6 _returnvalue_11) (|GetJsonField (Variables|Utility|GetControls) "cameraDownAmount")) ; Input froom JSON received
              (if _returnvalue_11
                (Variables|Utility|SetCameraPitchAxisValue _outvalue_6)
                ;;[1 1 1] Set all elements of array to false
                (for (_ _array_index_5) _branchisactive_5
                  (Utilities|Array|SetArrayElem _branchisactive_5 _array_index_5 false))
                (Utilities|Array|SetArrayElem _branchisactive_5 4 true) ; Set the relevant array element to true
                (Timeline|ConstantTime PlayFromStart)))
            (:then_5
              ;[1 1 1] Hnadle Hover
              (bind (_outvalue_7 _returnvalue_12) (|GetJsonField (Variables|Utility|GetControls) "hover")) ; Input froom JSON received
              (if _returnvalue_12
                (if _outvalue_7
                  ;;[1 1 1] Set all elements of array to false
                  (for (_ _array_index_6) _branchisactive_6
                    (Utilities|Array|SetArrayElem _branchisactive_6 _array_index_6 false)))))
            (:then_6
              ;[1 1 1] Handle Rotating X Degrees at speed Y
              (bind (_outvalue_8 _returnvalue_13) (|GetJsonField (Variables|Utility|GetControls) "rotateXDegrees")) ; Input froom JSON received
              (if _returnvalue_13
                (bind (_outvalue_9 _returnvalue_14) (|GetJsonField (Variables|Utility|GetControls) "rotationSpeed")) ; Rotation speed (deg per sec) received
                (if _returnvalue_14
                  (Variables|Utility|SetRotationSpeed (/ 1.0 _outvalue_9))
                  (else
                    (Variables|Utility|SetRotationSpeed 0.011111) ; Default speed if none received: 90 deg per second or 1/90 of a sec per 1 degree
                  ))
                (Components|MoveComponentTo _quadcopterbox (.location _returnvalue_3) (Math|Rotator|MakeRotator (.roll (.rotation _returnvalue_3)) (.pitch (.rotation _returnvalue_3)) (+ (.yaw (.rotation _returnvalue_3)) _outvalue_8)) true true (* _outvalue_8 (Variables|Utility|GetRotationSpeed)) false)))
            (:then_7
              ;[1 1 1] Goto
              (bind (_outvalue_10 _returnvalue_15) (|GetJsonField (Variables|Utility|GetControls) "goto")) ; Input froom JSON received
              (if _returnvalue_15
                (bind (_outvalue_11 _returnvalue_16) (|GetJsonField _outvalue_10 "gotoXVal")) ; Target vector X
                (bind (_outvalue_12 _returnvalue_17) (|GetJsonField _outvalue_10 "gotoYVal")) ; Target vector Y
                (bind (_outvalue_13 _returnvalue_18) (|GetJsonField _outvalue_10 "gotoZVal")) ; Target vector Z
                (bind (_outvalue_14 _returnvalue_19) (|GetJsonField _outvalue_10 "gotoSpeed")) ; Speed of movement in m/s
                (bind (_outvalue_15 _returnvalue_20) (|GetJsonField _outvalue_10 "turnWithMove")) ; Turn with move bool value - determines if the drone will face the target location of goto (true), or continue facing the original direction (false)
                (if (Math|Boolean|ANDBoolean _returnvalue_20 _returnvalue_19 _returnvalue_18 _returnvalue_17 _returnvalue_16) ; Iff all these values exist
                  (if _outvalue_15 ; if turn with move == true
                    (Variables|Utility|SetGotoTurnVector (Math|Rotator|FindLookatRotation (Transformation|GetWorldLocation (Variables|Default|GetQuadcopterBox)) (Math|Vector|MakeVector _outvalue_11 _outvalue_12 _outvalue_13)))
                    (else
                      (Variables|Utility|SetGotoTurnVector (.rotation _returnvalue))))
                  (Components|MoveComponentTo (Variables|Default|GetQuadcopterBox) (Math|Vector|MakeVector _outvalue_11 _outvalue_12 _outvalue_13) (Variables|Utility|GetGotoTurnVector) true true (/ (Math|Vector|Distance(Vector) (.location _returnvalue) (Math|Vector|MakeVector _outvalue_11 _outvalue_12 _outvalue_13)) (* _outvalue_14 1e+02)) false))))
            (:then_8
              ;[1 1 1] Turn towards point XYZ at speed V
              (bind (_outvalue_16 _returnvalue_21) (|GetJsonField (Variables|Utility|GetControls) "turnTowards")) ; Input froom JSON received
              (if _returnvalue_21
                (bind (_outvalue_17 _returnvalue_22) (|GetJsonField _outvalue_16 "turnTowardsXVal")) ; Target vector X
                (bind (_outvalue_18 _returnvalue_23) (|GetJsonField _outvalue_16 "turnTowardsYVal")) ; Target vector Y
                (bind (_outvalue_19 _returnvalue_24) (|GetJsonField _outvalue_16 "turnTowardsZVal")) ; Target vector Z
                (if (Math|Boolean|ANDBoolean _returnvalue_24 _returnvalue_23 _returnvalue_22) ; Iff all these values exist
                  (bind (_outvalue_20 _returnvalue_25) (|GetJsonField _outvalue_16 "turnTowardsSpeed")) ; Speed of rotation
                  (if _returnvalue_25
                    (Variables|Utility|SetRotationSpeed (/ 1.0 _outvalue_20))
                    (else
                      (Variables|Utility|SetRotationSpeed 0.011111) ; Default speed if none received: 90 deg per second or 1/90 of a sec per 1 degree
                    ))
                  (Components|MoveComponentTo _quadcopterbox_3 _returnvalue_4 (Math|Rotator|MakeRotator 0.0 0.0 (.yaw (Math|Rotator|FindLookatRotation _returnvalue_4 (Math|Vector|MakeVector _outvalue_17 _outvalue_18 _outvalue_19)))) true true (* (Math|Float|Absolute(Float) (.yaw (Math|Rotator|FindLookatRotation _returnvalue_4 (Math|Vector|MakeVector _outvalue_17 _outvalue_18 _outvalue_19)))) (Variables|Utility|GetRotationSpeed)) false)))))))
      (:then_1
        (bind (_outvalue_21 _returnvalue_26) (|GetJsonField (Variables|Utility|GetInputJson) "getDroneState")) ; Drone state is requestede
        (if _returnvalue_26
          (if _outvalue_21
            (bind _outputjson (CallFunction|ConstructDroneState))
            (bind _outjsonstring (Class|JsonBlueprintFunctionLibrary|ToString _outputjson))
            (Class|UDPComponent|EmitBytes (Variables|Default|GetUDPComponent) (Class|CUBlueprintLibrary|ToBytes(String) _outjsonstring)) ; Sends message via UDP socket
          )))
      (:then_2
        (bind (_outvalue_22 _returnvalue_27) (|GetJsonField (Variables|Utility|GetInputJson) "droneGrade")) ; Drone grade is received
        (if _returnvalue_27
          (Development|PrintString (Utilities|String|Append "The current grade is: " _outvalue_22))))
      (:then_3
        (bind (_outvalue_23 _returnvalue_28) (|GetJsonField (Variables|Utility|GetInputJson) "getDistanceToCameraDirection")) ; Distance to point is requested
        (if _returnvalue_28
          (if _outvalue_23
            (bind _outhit (CallFunction|LineTracefromCamera))
            (Class|UDPComponent|EmitBytes (Variables|Default|GetUDPComponent) (Class|CUBlueprintLibrary|ToBytes(String) (Utilities|String|ToString(Float) (Math|Vector|Distance(Vector) (.Location (Collision|BreakHitResult _outhit)) (Transformation|GetWorldLocation (Variables|Default|GetQuadcopterBox)))))) ; Sends message via UDP socket
          ))))
    (else
      (Utilities|String|LogString "Error reading JSON string"))))

(event OnComponentHit(QuadcopterBox)
  (params (HitComponent :type Primitive%20Component%20Object%20Reference) (OtherActor :type Actor%20Object%20Reference) (OtherComp :type Primitive%20Component%20Object%20Reference) (NormalImpulse :type Vector :default "0, 0, 0") (Hit :type Hit%20Result%20Structure%20%28by%20ref%29))
  (Variables|ForOutput|SetCollisionCount (+ (Variables|ForOutput|GetCollisionCount) 1)))

(event Input|AxisEvents|InputAxisQuadThrottle
  (params (AxisValue :type Float%20%28single-precision%29))
  (bind _camerapitchaxisvalue (Variables|Utility|GetCameraPitchAxisValue))
  (bind _branchisactive (Variables|Utility|GetBranchIsActive))
  (bind _camera (Variables|Default|GetCamera))
  (bind _returnvalue (Transformation|GetWorldRotation _camera))
  (bind _returnvalue_2 (* _camerapitchaxisvalue 2.0))
  (bind _returnvalue_3 (+ _returnvalue_2 (.pitch _returnvalue)))
  ;[0.8565 1 0.7031] Momentary Controls of Quadcopter
  ;;[1 1 1] Handling Throttle
  (if (!= 0.0 AxisValue)
    (Variables|Utility|SetThrottleAxisValue AxisValue)
    ;;[1 1 1] Set all elements of array to false
    (for (_ _array_index) _branchisactive
      (Utilities|Array|SetArrayElem _branchisactive _array_index false))
    (Utilities|Array|SetArrayElem _branchisactive 0 true) ; Set the relevant array element to true
    (Timeline|ConstantTime PlayFromStart
      (:Update
        (if (Utilities|Array|Get(acopy) (Variables|Utility|GetBranchIsActive))
          ;;[1 1 1] Movement Control - Throttle
          (Class|PawnMovementComponent|AddInputVector (Variables|Default|GetFloatingPawnMovement) (* (Variables|Utility|GetThrottleAxisValue) (Math|Vector|VectorUp)) false)
          (elif (Utilities|Array|Get(acopy) (Variables|Utility|GetBranchIsActive) 1)
            ;;[1 1 1] Movement Control - Pitch
            (Class|PawnMovementComponent|AddInputVector (Variables|Default|GetFloatingPawnMovement) (* (Variables|Utility|GetPitchAxisValue) (Transformation|GetActorForwardVector)) false)
            (elif (Utilities|Array|Get(acopy) (Variables|Utility|GetBranchIsActive) 2)
              ;;[1 1 1] Movement Control - Roll
              (Class|PawnMovementComponent|AddInputVector (Variables|Default|GetFloatingPawnMovement) (* (Variables|Utility|GetRollAxisValue) (Transformation|GetActorRightVector)) false)
              (elif (Utilities|Array|Get(acopy) (Variables|Utility|GetBranchIsActive) 3)
                ;;[1 1 1] Movement Control - Yaw
                (Transformation|SetWorldRotation (Variables|Default|GetQuadcopterBox) (Math|Rotator|MakeRotator 0.0 0.0 (+ (* (Variables|Utility|GetYawAxisValue) 3.0) (.yaw (Transformation|GetWorldRotation (Variables|Default|GetQuadcopterBox))))) false false)
                (elif (Utilities|Array|Get(acopy) (Variables|Utility|GetBranchIsActive) 4)
                  ;;[1 1 1] Movement Control - Camera Pitch
                  (if (< (Math|Float|Absolute(Float) _returnvalue_3) 9e+01)
                    (Transformation|SetWorldRotation (Variables|Default|GetCamera) (Math|Rotator|MakeRotator (.roll _returnvalue) _returnvalue_3 (.yaw _returnvalue)) false false)))))))))))

(event Input|AxisEvents|InputAxisQuadPitch
  (params (AxisValue :type Float%20%28single-precision%29))
  (bind _camerapitchaxisvalue (Variables|Utility|GetCameraPitchAxisValue))
  (bind _branchisactive (Variables|Utility|GetBranchIsActive))
  (bind _camera (Variables|Default|GetCamera))
  (bind _returnvalue (Transformation|GetWorldRotation _camera))
  (bind _returnvalue_2 (* _camerapitchaxisvalue 2.0))
  (bind _returnvalue_3 (+ _returnvalue_2 (.pitch _returnvalue)))
  ;[0.8565 1 0.7031] Momentary Controls of Quadcopter
  ;;[1 1 1] Handling Pitch
  (if (!= 0.0 AxisValue)
    (Variables|Utility|SetPitchAxisValue AxisValue)
    ;;[1 1 1] Set all elements of array to false
    (for (_ _array_index) _branchisactive
      (Utilities|Array|SetArrayElem _branchisactive _array_index false))
    (Utilities|Array|SetArrayElem _branchisactive 1 true) ; Set the relevant array element to true
    (Timeline|ConstantTime PlayFromStart
      (:Update
        (if (Utilities|Array|Get(acopy) (Variables|Utility|GetBranchIsActive))
          ;;[1 1 1] Movement Control - Throttle
          (Class|PawnMovementComponent|AddInputVector (Variables|Default|GetFloatingPawnMovement) (* (Variables|Utility|GetThrottleAxisValue) (Math|Vector|VectorUp)) false)
          (elif (Utilities|Array|Get(acopy) (Variables|Utility|GetBranchIsActive) 1)
            ;;[1 1 1] Movement Control - Pitch
            (Class|PawnMovementComponent|AddInputVector (Variables|Default|GetFloatingPawnMovement) (* (Variables|Utility|GetPitchAxisValue) (Transformation|GetActorForwardVector)) false)
            (elif (Utilities|Array|Get(acopy) (Variables|Utility|GetBranchIsActive) 2)
              ;;[1 1 1] Movement Control - Roll
              (Class|PawnMovementComponent|AddInputVector (Variables|Default|GetFloatingPawnMovement) (* (Variables|Utility|GetRollAxisValue) (Transformation|GetActorRightVector)) false)
              (elif (Utilities|Array|Get(acopy) (Variables|Utility|GetBranchIsActive) 3)
                ;;[1 1 1] Movement Control - Yaw
                (Transformation|SetWorldRotation (Variables|Default|GetQuadcopterBox) (Math|Rotator|MakeRotator 0.0 0.0 (+ (* (Variables|Utility|GetYawAxisValue) 3.0) (.yaw (Transformation|GetWorldRotation (Variables|Default|GetQuadcopterBox))))) false false)
                (elif (Utilities|Array|Get(acopy) (Variables|Utility|GetBranchIsActive) 4)
                  ;;[1 1 1] Movement Control - Camera Pitch
                  (if (< (Math|Float|Absolute(Float) _returnvalue_3) 9e+01)
                    (Transformation|SetWorldRotation (Variables|Default|GetCamera) (Math|Rotator|MakeRotator (.roll _returnvalue) _returnvalue_3 (.yaw _returnvalue)) false false)))))))))))

(event Input|AxisEvents|InputAxisCameraPitch
  (params (AxisValue :type Float%20%28single-precision%29))
  (bind _branchisactive (Variables|Utility|GetBranchIsActive))
  (bind _camera (Variables|Default|GetCamera))
  (bind _returnvalue (Transformation|GetWorldRotation _camera))
  ;[0.8565 1 0.7031] Momentary Controls of Quadcopter
  ;;[1 1 1] Handle Camera Pitch
  (if (!= 0.0 AxisValue)
    (Variables|Utility|SetCameraPitchAxisValue AxisValue)
    ;;[1 1 1] Set all elements of array to false
    (for (_ _array_index) _branchisactive
      (Utilities|Array|SetArrayElem _branchisactive _array_index false))
    (Utilities|Array|SetArrayElem _branchisactive 4 true) ; Set the relevant array element to true
    (Timeline|ConstantTime PlayFromStart
      (:Update
        (if (Utilities|Array|Get(acopy) (Variables|Utility|GetBranchIsActive))
          ;;[1 1 1] Movement Control - Throttle
          (Class|PawnMovementComponent|AddInputVector (Variables|Default|GetFloatingPawnMovement) (* (Variables|Utility|GetThrottleAxisValue) (Math|Vector|VectorUp)) false)
          (elif (Utilities|Array|Get(acopy) (Variables|Utility|GetBranchIsActive) 1)
            ;;[1 1 1] Movement Control - Pitch
            (Class|PawnMovementComponent|AddInputVector (Variables|Default|GetFloatingPawnMovement) (* (Variables|Utility|GetPitchAxisValue) (Transformation|GetActorForwardVector)) false)
            (elif (Utilities|Array|Get(acopy) (Variables|Utility|GetBranchIsActive) 2)
              ;;[1 1 1] Movement Control - Roll
              (Class|PawnMovementComponent|AddInputVector (Variables|Default|GetFloatingPawnMovement) (* (Variables|Utility|GetRollAxisValue) (Transformation|GetActorRightVector)) false)
              (elif (Utilities|Array|Get(acopy) (Variables|Utility|GetBranchIsActive) 3)
                ;;[1 1 1] Movement Control - Yaw
                (Transformation|SetWorldRotation (Variables|Default|GetQuadcopterBox) (Math|Rotator|MakeRotator 0.0 0.0 (+ (* (Variables|Utility|GetYawAxisValue) 3.0) (.yaw (Transformation|GetWorldRotation (Variables|Default|GetQuadcopterBox))))) false false)
                (elif (Utilities|Array|Get(acopy) (Variables|Utility|GetBranchIsActive) 4)
                  ;;[1 1 1] Movement Control - Camera Pitch
                  (if (< (Math|Float|Absolute(Float) (+ (* (Variables|Utility|GetCameraPitchAxisValue) 2.0) (.pitch _returnvalue))) 9e+01)
                    (Transformation|SetWorldRotation (Variables|Default|GetCamera) (Math|Rotator|MakeRotator (.roll _returnvalue) (+ (* (Variables|Utility|GetCameraPitchAxisValue) 2.0) (.pitch _returnvalue)) (.yaw _returnvalue)) false false)))))))))))

(event Input|AxisEvents|InputAxisQuadYaw
  (params (AxisValue :type Float%20%28single-precision%29))
  (bind _camerapitchaxisvalue (Variables|Utility|GetCameraPitchAxisValue))
  (bind _branchisactive (Variables|Utility|GetBranchIsActive))
  (bind _camera (Variables|Default|GetCamera))
  (bind _returnvalue (Transformation|GetWorldRotation _camera))
  (bind _returnvalue_2 (* _camerapitchaxisvalue 2.0))
  (bind _returnvalue_3 (+ _returnvalue_2 (.pitch _returnvalue)))
  ;[0.8565 1 0.7031] Momentary Controls of Quadcopter
  ;;[1 1 1] Handle Yaw
  (if (!= 0.0 AxisValue)
    (Variables|Utility|SetYawAxisValue AxisValue)
    ;;[1 1 1] Set all elements of array to false
    (for (_ _array_index) _branchisactive
      (Utilities|Array|SetArrayElem _branchisactive _array_index false))
    (Utilities|Array|SetArrayElem _branchisactive 3 true) ; Set the relevant array element to true
    (Timeline|ConstantTime PlayFromStart
      (:Update
        (if (Utilities|Array|Get(acopy) (Variables|Utility|GetBranchIsActive))
          ;;[1 1 1] Movement Control - Throttle
          (Class|PawnMovementComponent|AddInputVector (Variables|Default|GetFloatingPawnMovement) (* (Variables|Utility|GetThrottleAxisValue) (Math|Vector|VectorUp)) false)
          (elif (Utilities|Array|Get(acopy) (Variables|Utility|GetBranchIsActive) 1)
            ;;[1 1 1] Movement Control - Pitch
            (Class|PawnMovementComponent|AddInputVector (Variables|Default|GetFloatingPawnMovement) (* (Variables|Utility|GetPitchAxisValue) (Transformation|GetActorForwardVector)) false)
            (elif (Utilities|Array|Get(acopy) (Variables|Utility|GetBranchIsActive) 2)
              ;;[1 1 1] Movement Control - Roll
              (Class|PawnMovementComponent|AddInputVector (Variables|Default|GetFloatingPawnMovement) (* (Variables|Utility|GetRollAxisValue) (Transformation|GetActorRightVector)) false)
              (elif (Utilities|Array|Get(acopy) (Variables|Utility|GetBranchIsActive) 3)
                ;;[1 1 1] Movement Control - Yaw
                (Transformation|SetWorldRotation (Variables|Default|GetQuadcopterBox) (Math|Rotator|MakeRotator 0.0 0.0 (+ (* (Variables|Utility|GetYawAxisValue) 3.0) (.yaw (Transformation|GetWorldRotation (Variables|Default|GetQuadcopterBox))))) false false)
                (elif (Utilities|Array|Get(acopy) (Variables|Utility|GetBranchIsActive) 4)
                  ;;[1 1 1] Movement Control - Camera Pitch
                  (if (< (Math|Float|Absolute(Float) _returnvalue_3) 9e+01)
                    (Transformation|SetWorldRotation (Variables|Default|GetCamera) (Math|Rotator|MakeRotator (.roll _returnvalue) _returnvalue_3 (.yaw _returnvalue)) false false)))))))))))

(event Input|AxisEvents|InputAxisQuadRoll
  (params (AxisValue :type Float%20%28single-precision%29))
  (bind _camerapitchaxisvalue (Variables|Utility|GetCameraPitchAxisValue))
  (bind _branchisactive (Variables|Utility|GetBranchIsActive))
  (bind _camera (Variables|Default|GetCamera))
  (bind _returnvalue (Transformation|GetWorldRotation _camera))
  (bind _returnvalue_2 (* _camerapitchaxisvalue 2.0))
  (bind _returnvalue_3 (+ _returnvalue_2 (.pitch _returnvalue)))
  ;[0.8565 1 0.7031] Momentary Controls of Quadcopter
  ;;[1 1 1] Handle Roll
  (if (!= 0.0 AxisValue)
    (Variables|Utility|SetRollAxisValue AxisValue)
    ;;[1 1 1] Set all elements of array to false
    (for (_ _array_index) _branchisactive
      (Utilities|Array|SetArrayElem _branchisactive _array_index false))
    (Utilities|Array|SetArrayElem _branchisactive 2 true) ; Set the relevant array element to true
    (Timeline|ConstantTime PlayFromStart
      (:Update
        (if (Utilities|Array|Get(acopy) (Variables|Utility|GetBranchIsActive))
          ;;[1 1 1] Movement Control - Throttle
          (Class|PawnMovementComponent|AddInputVector (Variables|Default|GetFloatingPawnMovement) (* (Variables|Utility|GetThrottleAxisValue) (Math|Vector|VectorUp)) false)
          (elif (Utilities|Array|Get(acopy) (Variables|Utility|GetBranchIsActive) 1)
            ;;[1 1 1] Movement Control - Pitch
            (Class|PawnMovementComponent|AddInputVector (Variables|Default|GetFloatingPawnMovement) (* (Variables|Utility|GetPitchAxisValue) (Transformation|GetActorForwardVector)) false)
            (elif (Utilities|Array|Get(acopy) (Variables|Utility|GetBranchIsActive) 2)
              ;;[1 1 1] Movement Control - Roll
              (Class|PawnMovementComponent|AddInputVector (Variables|Default|GetFloatingPawnMovement) (* (Variables|Utility|GetRollAxisValue) (Transformation|GetActorRightVector)) false)
              (elif (Utilities|Array|Get(acopy) (Variables|Utility|GetBranchIsActive) 3)
                ;;[1 1 1] Movement Control - Yaw
                (Transformation|SetWorldRotation (Variables|Default|GetQuadcopterBox) (Math|Rotator|MakeRotator 0.0 0.0 (+ (* (Variables|Utility|GetYawAxisValue) 3.0) (.yaw (Transformation|GetWorldRotation (Variables|Default|GetQuadcopterBox))))) false false)
                (elif (Utilities|Array|Get(acopy) (Variables|Utility|GetBranchIsActive) 4)
                  ;;[1 1 1] Movement Control - Camera Pitch
                  (if (< (Math|Float|Absolute(Float) _returnvalue_3) 9e+01)
                    (Transformation|SetWorldRotation (Variables|Default|GetCamera) (Math|Rotator|MakeRotator (.roll _returnvalue) _returnvalue_3 (.yaw _returnvalue)) false false)))))))))))

(fn ConstructionScript)

(fn ConstructDroneState
  (bind _outputjson (Variables|Utility|GetOutputJson))
  (bind _quadcopterbox (Variables|Default|GetQuadcopterBox))
  (bind _returnvalue (Transformation|GetWorldLocation _quadcopterbox))
  (|SetJsonField _outputjson "collisionCount" (Variables|ForOutput|GetCollisionCount))
  ;[1 1 1] Position
  (|SetJsonField _outputjson "positionXVal" (.x _returnvalue))
  (|SetJsonField _outputjson "positionYVal" (.y _returnvalue))
  (|SetJsonField _outputjson "positionZVal" (.z _returnvalue))
  (return _outputjson))

(fn LineTracefromCamera
  (bind _camera (Variables|Default|GetCamera))
  (bind _returnvalue (Transformation|GetWorldLocation _camera))
  (bind (_outhit _returnvalue_2) (Collision|LineTraceForObjects _returnvalue (+ _returnvalue (* (Math|Vector|GetForwardVector _camera) 1e+04)) (Utilities|Array|MakeArray "ObjectTypeQuery1" "ObjectTypeQuery4" "ObjectTypeQuery2") false 0 "None"))
  (return _outhit _returnvalue_2))